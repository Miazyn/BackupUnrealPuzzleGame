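; BP_Lillypad is a lily pad platform that sinks and resurfaces when the first-person character enters its detection box.
; Fake pads drop immediately on overlap, while real pads wait for a delay before dropping; both rise again after another delay.
; LillyDown and LillyUp move the actor instantly by a Z offset, and DoOnce gates block retriggering until each cycle finishes.
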(event OnComponentBeginOverlap(Detectionbox)
  (params (OverlappedComponent :type Primitive%20Component%20Object%20Reference) (OtherActor :type Actor%20Object%20Reference) (OtherComp :type Primitive%20Component%20Object%20Reference) (OtherBodyIndex :type Integer) (bFromSweep :type Boolean) (SweepResult :type Hit%20Result%20Structure%20%28by%20ref%29))
  (Utilities|Casting|CastToBP_FirstPersonCharacter OtherActor)
  (if (Variables|Default|GetIsFake?)
    (Utilities|FlowControl|DoOnce false :!label _label
      (:Completed
        (CallFunction|LillyDown)
        (Utilities|FlowControl|Delay (Variables|Default|GetDelay))
        (CallFunction|LillyUp)
        (goto _label Reset)))
    (else
      (Utilities|FlowControl|DoOnce false :!label _label_2
        (:Completed
          (Utilities|FlowControl|Delay (Variables|Default|GetDelay))
          (CallFunction|LillyDown)
          (Utilities|FlowControl|Delay (Variables|Default|GetDelay))
          (CallFunction|LillyUp)
          (goto _label_2 Reset))))))

(event Custom|LillyUp
  (bind _returnvalue (Transformation|GetActorLocation))
  (Transformation|SetActorLocation (Math|Vector|MakeVector (.x _returnvalue) (.y _returnvalue) (+ (.z _returnvalue) (Variables|Default|GetOffset))) false false)
  (Development|PrintString "Up"))

(event Custom|LillyDown
  (bind _returnvalue (Transformation|GetActorLocation))
  (Transformation|SetActorLocation (Math|Vector|MakeVector (.x _returnvalue) (.y _returnvalue) (- (.z _returnvalue) (Variables|Default|GetOffset))) false false)
  (Development|PrintString "Down"))

(fn ConstructionScript)