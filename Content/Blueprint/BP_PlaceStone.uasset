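; BP_PlaceStone is a placement spot that automatically slots one designated stone (Stein) into position.
; When that BP_Stein overlaps the Box, a MoveComponentTo latent action eases its mesh over one second to this actor's location and a fixed rotation, and physics simulation is switched off.
; A one-second timer calls StopMoving to halt the move, while normal completion prints a confirmation string.
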(event OnComponentBeginOverlap(Box)
  (params (OverlappedComponent :type Primitive%20Component%20Object%20Reference) (OtherActor :type Actor%20Object%20Reference) (OtherComp :type Primitive%20Component%20Object%20Reference) (OtherBodyIndex :type Integer) (bFromSweep :type Boolean) (SweepResult :type Hit%20Result%20Structure%20%28by%20ref%29))
  ;[0.151 0.151 0.151] Stein an die Richtige stelle automatisch platzieren lassen
  (bind _asbp_stein (Utilities|Casting|CastToBP_Stein OtherActor))
  (if (== OtherActor (Variables|Default|GetStein))
    (CallFunction|MovetoEnd)
    (Physics|SetSimulatePhysics (Variables|/Game/Blueprint/BP_Stein.BP_Stein_C|GetStaticMesh _asbp_stein) false)
    (Utilities|Time|SetTimerbyFunctionName 0 "StopMoving" 1.0)))

(event Custom|MoveToEnd
  ;[0.151 0.151 0.151] Stein an die Richtige stelle automatisch platzieren lassen
  (Components|MoveComponentTo (Variables|/Game/Blueprint/BP_Stein.BP_Stein_C|GetStaticMesh (stale OnComponentBeginOverlap(Box) _asbp_stein)) (Transformation|GetActorLocation) "0.000000,90.000000,0.000000" false false 1.0 false)
  (Development|PrintString "Stone Placed!"))

(event Custom|StopMoving
  ;[0.151 0.151 0.151] Stein an die Richtige stelle automatisch platzieren lassen
  (Components|MoveComponentTo (Variables|/Game/Blueprint/BP_Stein.BP_Stein_C|GetStaticMesh (stale OnComponentBeginOverlap(Box) _asbp_stein)) (Transformation|GetActorLocation) "0.000000,90.000000,0.000000" false false 1.0 false) ; enters at Stop
)

(event EventBeginPlay)

(event Collision|EventActorBeginOverlap
  (params (OtherActor :type Actor%20Object%20Reference)))

(event EventTick
  (params (DeltaSeconds :type Float%20%28single-precision%29)))

(fn ConstructionScript)