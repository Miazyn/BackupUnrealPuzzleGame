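; BP_Zahnrad is a gear that spins on its pitch axis until stopped, which, per its comment, happens through interacting with plants.
; Tick applies the Rotation speed scaled by delta time.
; StopRotate zeroes that speed and, once only, increments a deactivation counter, opens the referenced Door when it equals one, and plays the ChangeColor timeline.
; That timeline tints a dynamic material created in the construction script.
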(event Custom|StopRotate
  ;[0.04706 0.1961 0.03529] Zahnrad wird gestoppt indem man mit pflanzen interagiert
  (Development|PrintString "Zahnrad gestoppt")
  (Transformation|AddActorLocalRotation (Math|Rotator|MakeRotator 0.0 (* (stale _output_get) 0.0) 0.0) false false)
  (bind _output_get (Variables|Default|SetRotation 0.0))
  (Utilities|FlowControl|DoOnce false
    (:Completed
      (Variables|Default|SetZahnradDeaktiviert (+ (Variables|Default|GetZahnradDeaktiviert) 1))
      (if (== (Variables|Default|GetZahnradDeaktiviert) 1)
        (Default|OpenDoor (Variables|Default|GetDoor))
        (bind _colorchange (Timeline|ChangeColor Play)
          (:Update
            (Rendering|Material|SetVectorParameterValue (Variables|Default|GetMaterial) "ChangeColor" _colorchange :!class /Script/Engine.MaterialInstanceDynamic)))))))

(event EventBeginPlay)

(event Collision|EventActorBeginOverlap
  (params (OtherActor :type Actor%20Object%20Reference)))

(event EventTick
  (params (DeltaSeconds :type Float%20%28single-precision%29))
  ;[0.1771 0.1771 0.1771] Zahnrad Rotation
  (Transformation|AddActorLocalRotation (Math|Rotator|MakeRotator 0.0 (* (Variables|Default|GetRotation) DeltaSeconds) 0.0) false false))

(fn ConstructionScript
  (bind _returnvalue (Rendering|Material|CreateDynamicMaterialInstance (Variables|Default|GetZahnrad) 0 0 "None" :!class /Script/Engine.PrimitiveComponent))
  (Variables|Default|SetMaterial _returnvalue))